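; BananaCollectorPlayer is the player actor for what appears to be a banana-collecting game, and handles only its movement.
; MoveHorizontal and MoveVertical axes add movement input along the actor's right and forward vectors.
; Tick consumes that input, clamps its length to one so diagonals are no faster, and scales it by MaxSpeed and delta time.
; The result is applied as an unswept local offset, although the input is in world space.
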(event EventBeginPlay)

(event Collision|EventActorBeginOverlap
  (params (OtherActor :type Actor%20Object%20Reference)))

(event EventTick
  (params (DeltaSeconds :type Float%20%28single-precision%29))
  (bind _returnvalue (Class|Pawn|ConsumeMovementInputVector))
  (Transformation|AddActorLocalOffset (* (Math|Vector|ClampVectorSize _returnvalue 0.0 1.0) (* DeltaSeconds (Variables|Default|GetMaxSpeed))) false false))

(event Input|ActionEvents|InputActionJump
  (params (Key :type Key%20Structure :default "None")))

(event Input|AxisEvents|InputAxisMoveHorizontal
  (params (AxisValue :type Float%20%28single-precision%29))
  (Pawn|Input|AddMovementInput (* (Transformation|GetActorRightVector) AxisValue) 1.0 false))

(event Input|AxisEvents|InputAxisMoveVertical
  (params (AxisValue :type Float%20%28single-precision%29))
  (Pawn|Input|AddMovementInput (* (Transformation|GetActorForwardVector) AxisValue) 1.0 false))

(fn ConstructionScript)